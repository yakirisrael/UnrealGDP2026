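; BP_MovableCube is an elevator actor whose cube moves vertically, with a sphere area that detects the player.
; Sphere overlap sets the player BP_ThirdPersonCharacter's Elevator reference to this actor and clears it on exit, printing debug messages.
; TurnOnElevator, not triggered within this Blueprint, saves the cube's start location and plays a timeline.
; Each timeline update applies its curve, scaled by MaxHeight, as a Z offset from that start.
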(event `self.ReceiveBeginPlay`)

(event `TurnOnElevator`
  ;[0.2763 0 0.3113 0.5] Need to save the start location before apply the offset per tick
  (set `self.StartLocation` (`SceneComponent.K2_GetComponentLocation` (`self.Cube`)))
  (bind (_direction _zoffset) (`Timeline|Elevator` :!via `PlayFromStart`)
    (:`Update`
      (`KismetSystemLibrary.PrintString` (`KismetStringLibrary.Conv_DoubleToString` _zoffset))
      (`self.AddZOffset` (* _zoffset (`self.MaxHeight`))))))

(event `self.Sphere1.OnComponentBeginOverlap`
  (params (OverlappedComponent :type "PrimitiveComponent Object Reference") (OtherActor :type "Actor Object Reference") (OtherComp :type "PrimitiveComponent Object Reference") (OtherBodyIndex :type Integer) (bFromSweep :type Boolean) (SweepResult :type "HitResult Structure (by ref)"))
  (bind _returnvalue (`GameplayStatics.GetPlayerPawn` 0))
  (if (== OtherActor _returnvalue)
    (set `self.InSphereArea` true)
    (bind _asbp_third_person_character (cast `/Game/ThirdPerson/Blueprints/BP_ThirdPersonCharacter` _returnvalue)
      (:`then`
        (set `/Game/ThirdPerson/Blueprints/BP_ThirdPersonCharacter.Elevator` self _asbp_third_person_character)
        (`KismetSystemLibrary.PrintString` (`KismetSystemLibrary.GetDisplayName` self) true true (struct :`R` 1.0 :`B` 0.126871 :`A` 1.0) 30.0))
      (:`CastFailed`
        (`KismetSystemLibrary.PrintString` "Not a third person character")))))

(event `self.Sphere1.OnComponentEndOverlap`
  (params (OverlappedComponent :type "PrimitiveComponent Object Reference") (OtherActor :type "Actor Object Reference") (OtherComp :type "PrimitiveComponent Object Reference") (OtherBodyIndex :type Integer))
  (bind _returnvalue (`GameplayStatics.GetPlayerPawn` 0))
  (if (== OtherActor _returnvalue)
    (set `self.InSphereArea` false)
    (bind _asbp_third_person_character (cast `/Game/ThirdPerson/Blueprints/BP_ThirdPersonCharacter` _returnvalue))
    (set `/Game/ThirdPerson/Blueprints/BP_ThirdPersonCharacter.Elevator` null _asbp_third_person_character)
    (`KismetSystemLibrary.PrintString` "go out of the elevator" true true (struct :`R` 0.085302 :`G` 1.0 :`B` 0.003172 :`A` 1.0) 30.0)))

(fn `AddZOffset`
  (params (Offset :type "Float (double-precision)"))
  (bind (_startlocation_x _startlocation_y _startlocation_z) (`KismetMathLibrary.BreakVector` (`self.StartLocation`)))
  (`SceneComponent.K2_SetWorldLocation` (`self.Cube`) (`KismetMathLibrary.MakeVector` _startlocation_x _startlocation_y (+ _startlocation_z Offset)) false false))

(fn `UserConstructionScript`)