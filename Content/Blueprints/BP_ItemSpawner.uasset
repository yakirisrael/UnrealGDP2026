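; Item spawner actor that spawns a BP_Key at its own location on BeginPlay, initialized from the "Key" row of DT_Items.
; It stores the key and starts a looping timer, using the row's Duration as interval, that only prints a debug message.
; Disconnected test logic remains for printing row data, bulk-spawning BP_Item through SpawnItems and destroying the key after a delay.
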(event `CustomEvent`
  (`KismetSystemLibrary.PrintString` "Key event"))

(event `self.ReceiveBeginPlay`
  (bind _returnvalue (`|GetDataTableRow` "/Game/Blueprints/Struct/DT_Items.DT_Items" "Key")
    (:`then`
      (bind _returnvalue_2 (`|SpawnActorFromClass` "/Game/Blueprints/BP_Key.BP_Key_C" (`KismetMathLibrary.MakeTransform` (`self.K2_GetActorLocation`)) "AlwaysSpawn" "MultiplyWithRoot" null _returnvalue null))
      (set `self.Key` _returnvalue_2)
      (bind (_data_score _data_type _data_duration) (break `/Game/Blueprints/Struct/ST_ItemData` (`/Game/Blueprints/BP_Item.Data` _returnvalue_2)))
      (bind _returnvalue_3 (`KismetSystemLibrary.K2_SetTimerDelegate` (delegate `CustomEvent`) _data_duration true))
      (set `self.Timer` _returnvalue_3))))

(fn `SpawnItems`
  (for _ (range 1 101)
    (`|SpawnActorFromClass` "/Game/Blueprints/BP_Item.BP_Item_C" (`KismetMathLibrary.MakeTransform` (`self.K2_GetActorLocation`)) "AlwaysSpawn" "MultiplyWithRoot" null (struct) null)))

(fn `UserConstructionScript`)