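; BP_WeaponBase is a weapon actor that works as both a world pickup and a bullet-firing gun.
; When the player pawn overlaps PickupTrigger, it passes its WeaponType to BP_ThirdPersonCharacter's PickupWeapon and destroys itself.
; DisableTrigger turns off the trigger's collision.
; Shoot spawns a scaled-down BP_Bullet at BarrelEdge and launches it with a physics impulse along the barrel's forward vector.
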(event `DisableTrigger`
  (`PrimitiveComponent.SetCollisionEnabled` (`self.PickupTrigger`) "NoCollision"))

(event `Shoot`
  (bind _returnvalue (`|SpawnActorFromClass` "/Game/Blueprints/BP_Bullet.BP_Bullet_C" (`KismetMathLibrary.MakeTransform` (`SceneComponent.K2_GetComponentLocation` (`self.BarrelEdge`)) (struct) (0.05 0.05 0.05)) "AlwaysSpawn" "MultiplyWithRoot" null null))
  (bind _sphere (`/Game/Blueprints/BP_Bullet.Sphere` _returnvalue))
  (`PrimitiveComponent.SetSimulatePhysics` _sphere true)
  (`PrimitiveComponent.AddImpulse` _sphere (* (`SceneComponent.GetForwardVector` (`self.BarrelEdge`)) 2.0) "None" false))

(event `self.PickupTrigger.OnComponentBeginOverlap`
  (params (OverlappedComponent :type "PrimitiveComponent Object Reference") (OtherActor :type "Actor Object Reference") (OtherComp :type "PrimitiveComponent Object Reference") (OtherBodyIndex :type Integer) (bFromSweep :type Boolean) (SweepResult :type "HitResult Structure (by ref)"))
  (bind _returnvalue (`GameplayStatics.GetPlayerPawn` 0))
  (if (== OtherActor _returnvalue)
    (bind _asbp_third_person_character (cast `/Game/ThirdPerson/Blueprints/BP_ThirdPersonCharacter` _returnvalue))
    (`/Game/ThirdPerson/Blueprints/BP_ThirdPersonCharacter.PickupWeapon` _asbp_third_person_character (`self.WeaponType`))
    (`self.K2_DestroyActor`)))

(fn `UserConstructionScript`)