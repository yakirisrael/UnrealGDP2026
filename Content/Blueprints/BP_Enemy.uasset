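; Enemy Blueprint with a health bar widget that appears only while the player is inside its UI_Range trigger.
; On BeginPlay it hides the bar and plays a Timeline that sets actor yaw to the look-at angle toward the player, scaled by the curve value.
; Tick passes a small negative change to the health bar widget every frame.
; AI move-to and repeating jump logic are present but unconnected.
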(event `self.ReceiveBeginPlay`
  (bind (_returnvalue_roll _returnvalue_pitch) (`KismetMathLibrary.BreakRotator` (`self.K2_GetActorRotation`)))
  (bind (_returnvalue_roll_2 _returnvalue_pitch_2 _returnvalue_yaw) (`KismetMathLibrary.BreakRotator` (`KismetMathLibrary.FindLookAtRotation` (`SceneComponent.K2_GetComponentLocation` (`self.Mesh`)) (`self.K2_GetActorLocation` (`GameplayStatics.GetPlayerPawn` 0)))))
  (`self.Hide HealthBar`)
  (bind (_direction _deltaz) (`Timeline|Timeline` :!via `PlayFromStart`)
    (:`Update`
      (`self.K2_SetActorRotation` (`KismetMathLibrary.MakeRotator` _returnvalue_roll _returnvalue_pitch (* _deltaz _returnvalue_yaw))))))

(event `self.ReceiveTick`
  (params (DeltaSeconds :type "Float (single-precision)"))
  (bind _aswbp_health_bar (cast `/Game/Blueprints/UI/WBP_HealthBar` (`WidgetComponent.GetWidget` (`self.HealthBarWidget`))))
  (`/Game/Blueprints/UI/WBP_HealthBar.ChangeHP` _aswbp_health_bar -0.01))

(event `self.UI_Range.OnComponentBeginOverlap`
  (params (OverlappedComponent :type "PrimitiveComponent Object Reference") (OtherActor :type "Actor Object Reference") (OtherComp :type "PrimitiveComponent Object Reference") (OtherBodyIndex :type Integer) (bFromSweep :type Boolean) (SweepResult :type "HitResult Structure (by ref)"))
  (if (== OtherActor (`GameplayStatics.GetPlayerPawn` 0))
    (`self.Show HealthBar`)))

(event `self.UI_Range.OnComponentEndOverlap`
  (params (OverlappedComponent :type "PrimitiveComponent Object Reference") (OtherActor :type "Actor Object Reference") (OtherComp :type "PrimitiveComponent Object Reference") (OtherBodyIndex :type Integer))
  (if (== OtherActor (`GameplayStatics.GetPlayerPawn` 0))
    (`self.Hide HealthBar`)))

(fn `Hide HealthBar`
  (`SceneComponent.SetHiddenInGame` (`self.HealthBarWidget`) true true))

(fn `Show HealthBar`
  (`SceneComponent.SetHiddenInGame` (`self.HealthBarWidget`) false true))

(fn `UserConstructionScript`)